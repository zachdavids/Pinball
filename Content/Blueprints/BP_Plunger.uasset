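; BP_Plunger is an actor for a ball plunger that animates charge and release and supplies a ball spawn point.
; ChargePlunger plays a timeline that lerps the plunger mesh along local Y from its rest position.
; StopCharge halts the timeline and quickly moves the mesh with MoveComponentTo, with no explicit launch force.
; GetBallSpawnLocation converts the BallLocation offset to world space using the actor's transform.
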(event Custom|StopCharge
  (Utilities|FlowControl|Sequence
    (:then_0
      (bind _chargealpha (Timeline|ChargeTimeline Stop)
        (:Update
          (Transformation|SetRelativeLocation (Variables|Default|GetPlungerMesh) (Math|Vector|Lerp(Vector) "0, 0, 0" "0,150.000000,0.000000" _chargealpha) false false))))
    (:then_1
      (Components|MoveComponentTo (Variables|Default|GetPlungerMesh) "0, 0, 0" "0, 0, 0" false false 0.1 false))))

(event Custom|ChargePlunger
  (bind _chargealpha (Timeline|ChargeTimeline PlayFromStart)
    (:Update
      (Transformation|SetRelativeLocation (Variables|Default|GetPlungerMesh) (Math|Vector|Lerp(Vector) "0, 0, 0" "0,150.000000,0.000000" _chargealpha) false false))))

(fn ConstructionScript)

(fn GetBallSpawnLocation
  (return (Math|Transform|TransformLocation (Transformation|GetActorTransform) (Variables|Default|GetBallLocation))))